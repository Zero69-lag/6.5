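; A test Actor Blueprint that moves along a direction vector and bounces off whatever blocks it, losing speed with each hit.
; Tick applies a swept world offset from Dir and Speed, and a blocking hit reflects Dir about the surface normal with Z zeroed.
; Each hit prints Speed, then subtracts a fixed step, a tenth of the speed at BeginPlay, down to MinSpeed.
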(event `self.ReceiveBeginPlay`
  (set `self.umen` (* (`self.speed`) 0.1)))

(event `self.ReceiveTick`
  (params (DeltaSeconds :type "Float (single-precision)"))
  (bind _speed (`self.speed`))
  (bind _sweephitresult (`self.K2_AddActorWorldOffset` (* (* (`self.Dir`) (`self.speed`)) DeltaSeconds) true))
  (bind (_bblockinghit _binitialoverlap _time _distance _location _impactpoint _normal) (`GameplayStatics.BreakHitResult` _sweephitresult))
  (if _bblockinghit
    (bind (_returnvalue_x _returnvalue_y) (`KismetMathLibrary.BreakVector` (`KismetMathLibrary.GetReflectionVector` (`self.Dir`) _normal)))
    (set `self.Dir` (`KismetMathLibrary.MakeVector` _returnvalue_x _returnvalue_y))
    (`KismetSystemLibrary.PrintString` (`KismetStringLibrary.Conv_DoubleToString` _speed))
    (set `self.speed` (`KismetMathLibrary.FMax` (- _speed (`self.umen`)) (`self.min speed`)))))

(fn `UserConstructionScript`)