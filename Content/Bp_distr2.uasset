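; Bp_distr2 is an actor Blueprint that shrinks each time another actor begins to overlap it.
; On BeginPlay it stores a fixed fraction of its starting scale as DeltaScale.
; Each overlap runs the parent handler, then subtracts DeltaScale from the current scale, so the shrink is linear, with no lower limit.
; The construction script only calls the parent's.
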(event `self.ReceiveBeginPlay`
  (set `self.delta scale` (* (`self.GetActorScale3D`) 0.05)))

(event `self.ReceiveActorBeginOverlap`
  (params (OtherActor :type "Actor Object Reference"))
  (`parent.ReceiveActorBeginOverlap` OtherActor)
  (`self.SetActorScale3D` (- (`self.GetActorScale3D`) (`self.delta scale`))))

(fn `UserConstructionScript`
  (`parent.UserConstructionScript`))